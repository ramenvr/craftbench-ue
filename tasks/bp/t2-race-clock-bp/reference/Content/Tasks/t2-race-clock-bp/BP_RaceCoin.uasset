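; BP_RaceCoin is a pickup that awards points during a race round and then destroys itself.
; When a Character overlaps its CoinRegion, it finds the round actor through the RaceRound tag and reads RoundState from its RaceRoundBase parent class.
; Only while the round is InProgress does it pass PointValue to BP_RaceRound's AddPoints, with a Consumed flag guarding against repeat pickups.
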(event OnComponentBeginOverlap(CoinRegion)
  (params (OverlappedComponent :type Primitive%20Component%20Object%20Reference) (OtherActor :type Actor%20Object%20Reference) (OtherComp :type Primitive%20Component%20Object%20Reference) (OtherBodyIndex :type Integer) (bFromSweep :type Boolean) (SweepResult :type Hit%20Result%20Structure%20%28by%20ref%29))
  (if (not (Variables|Default|GetConsumed))
    (Utilities|Casting|CastToCharacter OtherActor)
    (bind _outactors (Actor|GetAllActorswithTag "RaceRound"))
    (if (Utilities|IsValid (Utilities|Array|Get(acopy) _outactors))
      (bind _asrace_round_base (Utilities|Casting|CastToRaceRoundBase (Utilities|Array|Get(acopy) _outactors)))
      (if (Utilities|Enum|Equal(Enum) (Variables|/Script/ThirdPerson.RaceRoundBase|GetRoundState _asrace_round_base) "InProgress")
        (bind _asbp_race_round (Utilities|Casting|CastToBP_RaceRound (Utilities|Array|Get(acopy) _outactors)))
        (Default|AddPoints _asbp_race_round (Variables|Default|GetPointValue))
        (Variables|Default|SetConsumed true)
        (Actor|DestroyActor)))))

(fn ConstructionScript)