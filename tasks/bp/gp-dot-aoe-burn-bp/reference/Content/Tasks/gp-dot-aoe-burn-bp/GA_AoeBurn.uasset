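; GA_AoeBurn is a Gameplay Ability that applies an area burn effect around its avatar.
; After a successful commit, it sphere-overlaps pawns of class CraftBenchCharacter at the avatar's location, without explicitly excluding the caster.
; It converts the results to target data and applies a GE_AoeBurnTick spec to them.
; The ability ends immediately afterward or when commit fails, leaving any ongoing burn to the effect.
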(event Ability|EventActivateAbility
  (bind _returnvalue (Ability|CommitAbility))
  (if _returnvalue
    (bind _outactors (Collision|SphereOverlapActors (Transformation|GetActorLocation (Ability|GetAvatarActorfromActorInfo)) 5e+02 (Utilities|Array|MakeArray "ObjectTypeQuery3") "/Script/ThirdPerson.CraftBenchCharacter"))
    (GameplayEffects|ApplyGameplayEffectSpecToTarget (Ability|MakeOutgoingGameplayEffectSpec "/Game/Tasks/gp-dot-aoe-burn-bp/GE_AoeBurnTick.GE_AoeBurnTick_C") (Ability|TargetData|AbilityTargetDatafromActorArray _outactors))
    (Ability|EndAbility)
    (else
      (Ability|EndAbility))))

(event Ability|EventOnEndAbility
  (params (bWasCancelled :type Boolean)))