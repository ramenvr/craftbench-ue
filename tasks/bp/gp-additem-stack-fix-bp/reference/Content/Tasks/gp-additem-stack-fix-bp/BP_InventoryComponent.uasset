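; Inventory component that tracks how many of each item its owner holds, along with a count of distinct item stacks.
; AddItem adds the amount to an existing entry in the Items map, or creates a new entry and increments StackCount.
; GetItemCount and GetStackCount expose those values, with no removal logic or stack size limit in these graphs.
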(event EventBeginPlay)

(event EventTick
  (params (DeltaSeconds :type Float%20%28single-precision%29)))

(fn AddItem
  (params (ItemId :type Name) (Count :type Integer))
  (bind _items (Variables|Default|GetItems))
  (if (Utilities|Map|Contains _items ItemId)
    (Utilities|Map|Add _items ItemId (+ (.Value (Utilities|Map|Find _items ItemId)) Count))
    (else
      (Utilities|Map|Add _items ItemId Count)
      (Variables|Default|SetStackCount (+ (Variables|Default|GetStackCount) 1)))))

(fn GetItemCount
  (params (ItemId :type Name))
  (return (.Value (Utilities|Map|Find (Variables|Default|GetItems) ItemId))))

(fn GetStackCount
  (return (Variables|Default|GetStackCount)))