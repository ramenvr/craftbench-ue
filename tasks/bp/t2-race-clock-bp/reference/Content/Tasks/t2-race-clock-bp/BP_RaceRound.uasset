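; BP_RaceRound is a race round scoreboard actor showing score, countdown and state, yawed each tick to face the player.
; Tick derives remaining time from game time since the round started, switching the state to TimedOut at zero.
; After timeout, pressing the tagged RaceReplayPad restarts the round, but only once the pad has been seen released, so a held press cannot retrigger.
; AddPoints increases the score and refreshes the text.
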(event EventBeginPlay
  (Variables|Default|SetRoundLength (Variables|Default|GetTimeRemaining))
  (bind _outactors (Actor|GetAllActorswithTag "RaceReplayPad"))
  (if (Utilities|IsValid (Utilities|Array|Get(acopy) _outactors))
    (Variables|Default|SetReplayPad (Utilities|Array|Get(acopy) _outactors))
    (CallFunction|RefreshReadouts)))

(event EventTick
  (params (DeltaSeconds :type Float%20%28single-precision%29))
  (bind _returnvalue (Utilities|Time|GetTimeSeconds))
  (bind _roundstartedat (Variables|Default|GetRoundStartedAt))
  (bind _roundlength (Variables|Default|GetRoundLength))
  (bind _replaypad (Variables|Default|GetReplayPad))
  (bind _returnvalue_2 (- _returnvalue _roundstartedat))
  (bind _returnvalue_3 (- _roundlength _returnvalue_2))
  (bind _returnvalue_4 (> _returnvalue_3 0.0))
  (Variables|Default|SetTimeRemaining (Math|Float|Max(Float) _returnvalue_3 0.0))
  (Variables|Default|SetRoundState (select _returnvalue_4 "InProgress" "TimedOut"))
  (CallFunction|RefreshReadouts)
  (CallFunction|FacetheWatcher)
  (if (not _returnvalue_4)
    (Utilities|IsValid _replaypad
      (:Is%20Valid
        (bind _asrace_replay_pad_actor (Utilities|Casting|CastToRaceReplayPadActor _replaypad))
        (if (Class|RaceReplayPadActor|IsPressed _asrace_replay_pad_actor)
          (if (Variables|Default|GetReplayArmed)
            (CallFunction|StartFreshRound))
          (else
            (Variables|Default|SetReplayArmed true)))))))

(fn ConstructionScript)

(fn RefreshReadouts
  (Rendering|Components|TextRender|SetText (Variables|Default|GetScoreText) (Utilities|Text|FormatText "SCORE {n}" (Variables|Default|GetScore)))
  (Rendering|Components|TextRender|SetText (Variables|Default|GetClockText) (Utilities|Text|ToText(String) (Utilities|String|ToString(Integer) (Math|Float|Ceil (Variables|Default|GetTimeRemaining)))))
  (Rendering|Components|TextRender|SetText (Variables|Default|GetStateText) (Utilities|Text|ToText(String) (Variables|Default|GetRoundState))))

(fn FacetheWatcher
  (bind _returnvalue (Game|Player|GetPlayerPawn 0))
  (Utilities|IsValid _returnvalue
    (:Is%20Valid
      (Transformation|SetActorRotation (Math|Rotator|MakeRotator 0.0 0.0 (.Yaw (Math|Rotator|BreakRotator (Math|Rotator|FindLookatRotation (Transformation|GetActorLocation) (Transformation|GetActorLocation _returnvalue)))))))))

(fn StartFreshRound
  (Variables|Default|SetScore 0)
  (Variables|Default|SetTimeRemaining (Variables|Default|GetRoundLength))
  (Variables|Default|SetRoundState "InProgress")
  (Variables|Default|SetRoundStartedAt (Utilities|Time|GetTimeSeconds))
  (Variables|Default|SetReplayArmed false)
  (CallFunction|RefreshReadouts))

(fn AddPoints
  (params (Points :type Integer))
  (Variables|Default|SetScore (+ (Variables|Default|GetScore) Points))
  (CallFunction|RefreshReadouts))