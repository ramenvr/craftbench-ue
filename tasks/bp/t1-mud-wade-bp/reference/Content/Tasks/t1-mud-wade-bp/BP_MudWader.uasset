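; BP_MudWader is a character that slows down and plays a looping wade animation while inside a mud patch.
; Each Tick scans actors tagged MudPatch and tests its location against their X/Y bounds, ignoring height, with no overlap events.
; An IsWading flag fires EnterMud and LeaveMud only on transitions.
; EnterMud scales down the walk speed cached at BeginPlay; LeaveMud restores it and the animation Blueprint.
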(event Custom|EnterMud
  (Variables|/Script/Engine.CharacterMovementComponent|SetMaxWalkSpeed (Variables|Character|GetCharacterMovement) (* (Variables|Default|GetOrdinaryTopSpeed) 0.4))
  (Components|Animation|PlayAnimation (Variables|Character|GetMesh) (Variables|Default|GetWadeMotion) true)
  (Variables|Default|SetIsWading true))

(event Custom|LeaveMud
  (bind _mesh (Variables|Character|GetMesh))
  (Variables|/Script/Engine.CharacterMovementComponent|SetMaxWalkSpeed (Variables|Character|GetCharacterMovement) (Variables|Default|GetOrdinaryTopSpeed))
  (Components|SkeletalMesh|SetAnimInstanceClass _mesh (Variables|/Script/Engine.SkeletalMeshComponent|GetAnimClass _mesh))
  (Variables|Default|SetIsWading false))

(event EventTick
  (params (DeltaSeconds :type Float%20%28single-precision%29))
  (bind _iswading (Variables|Default|GetIsWading))
  (Variables|Default|SetOnMud false)
  (bind _outactors (Actor|GetAllActorswithTag "MudPatch"))
  (bind _array_element (Utilities|Array|ForEachLoopwithBreak _outactors :!label _label)
    (:LoopBody
      (if (and (<= (Math|Float|Absolute(Float) (.X (Math|Vector|BreakVector (- (Transformation|GetActorLocation) (.Origin (Collision|GetActorBounds _array_element true false)))))) (.X (Math|Vector|BreakVector (.BoxExtent (Collision|GetActorBounds _array_element true false))))) (<= (Math|Float|Absolute(Float) (.Y (Math|Vector|BreakVector (- (Transformation|GetActorLocation) (.Origin (Collision|GetActorBounds _array_element true false)))))) (.Y (Math|Vector|BreakVector (.BoxExtent (Collision|GetActorBounds _array_element true false))))))
        (Variables|Default|SetOnMud true)
        (goto _label Break)))
    (:Completed
      (if (Variables|Default|GetOnMud)
        (if (not _iswading)
          (CallFunction|EnterMud))
        (elif _iswading
          (CallFunction|LeaveMud))))))

(event EventBeginPlay
  (Variables|Default|SetOrdinaryTopSpeed (Variables|/Script/Engine.CharacterMovementComponent|GetMaxWalkSpeed (Variables|Character|GetCharacterMovement))))

(fn ConstructionScript)