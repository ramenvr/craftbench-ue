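; BP_TintScreen is an actor that drives a vignette value from how fast the first player's character moves.
; Each Tick, it divides the character's velocity length by MaxWalkSpeed, guarding against an invalid character or zero speed.
; The clamped ratio blends RestVignette toward FullVignette and feeds SetVignette.
; The graph shows no color tint or post-process component, only that value update.
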(event EventBeginPlay)

(event Collision|EventActorBeginOverlap
  (params (OtherActor :type Actor%20Object%20Reference)))

(event EventTick
  (params (DeltaSeconds :type Float%20%28single-precision%29))
  (bind _returnvalue (Game|GetPlayerCharacter 0))
  (bind _charactermovement (Variables|/Script/Engine.Character|GetCharacterMovement _returnvalue))
  (bind _maxwalkspeed (Variables|/Script/Engine.CharacterMovementComponent|GetMaxWalkSpeed _charactermovement))
  (Utilities|IsValid _returnvalue
    (:Is%20Valid
      (if (> _maxwalkspeed 0.0)
        (Class|ScreenTintActor|SetVignette (Math|Float|Lerp (Variables|Default|GetRestVignette) (Variables|Default|GetFullVignette) (Math|Float|Clamp(Float) (/ (Math|Vector|VectorLength (Transformation|GetVelocity _returnvalue)) _maxwalkspeed))))))))

(fn ConstructionScript)