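; Yard barrier that opens when two named crates both rest on any of its pads.
; ShouldBeOpen requires both names to be home once either is set, deferring to the parent rule only when both are None.
; IsNamedCrateHome searches all YardCrateActors by name and tests each match against the valid pads.
; Tick reruns that check to light each lamp for the name its slot selects.
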(event EventTick
  (params (DeltaSeconds :type Float%20%28single-precision%29))
  (for _array_element (Variables|Default|GetLamps)
    (Utilities|IsValid _array_element
      (:Is%20Valid
        (bind _return_value (CallFunction|IsNamedCrateHome (select (== (Variables|/Script/ThirdPerson.GateLampActor|GetNameSlot _array_element) 0) (Variables|Default|GetCutForFirstName) (Variables|Default|GetCutForSecondName))))
        (Class|GateLampActor|SetLit _array_element _return_value)))))

(fn ConstructionScript)

(fn IsNamedCrateHome
  (params (Wanted%20Name :type Name))
  (if (Utilities|Name|NotEqual(Name) Wanted%20Name "None")
    (bind _outactors (Actor|GetAllActorsOfClass "/Script/ThirdPerson.YardCrateActor"))
    (for _array_element _outactors
      (bind _asyard_crate_actor (Utilities|Casting|CastToYardCrateActor _array_element))
      (if (Utilities|Name|Equal(Name) (Variables|/Script/ThirdPerson.YardCrateActor|GetCrateName _asyard_crate_actor) Wanted%20Name)
        (for _array_element_2 (Variables|Default|GetPads)
          (Utilities|IsValid _array_element_2
            (:Is%20Valid
              (if (Class|YardPadActor|IsBodyResting _array_element_2 _asyard_crate_actor)
                (return true))))))))
  (return false))

(fn ShouldbeOpen
  (bind _cutforfirstname (Variables|Default|GetCutForFirstName))
  (bind _cutforsecondname (Variables|Default|GetCutForSecondName))
  (if (or (Utilities|Name|NotEqual(Name) _cutforfirstname "None") (Utilities|Name|NotEqual(Name) _cutforsecondname "None"))
    (bind _return_value (CallFunction|IsNamedCrateHome _cutforfirstname))
    (bind _return_value_2 (CallFunction|IsNamedCrateHome _cutforsecondname))
    (return (and _return_value _return_value_2))
    (else
      (bind _returnvalue (|CallParentFunction))
      (return _returnvalue))))