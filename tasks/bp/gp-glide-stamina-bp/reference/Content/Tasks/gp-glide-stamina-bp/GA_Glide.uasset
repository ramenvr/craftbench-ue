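; GA_Glide is a Gameplay Ability that lets a character glide by limiting fall speed while applying a drain effect.
; On activation it commits, then starts a short looping timer for the glide tick, which is cleared when the ability ends.
; Each tick clamps downward velocity on CharacterMovement and applies GE_GlideDrain to the owner.
; The ability ends if commit fails or the checked attribute, unnamed in the graph, reaches zero.
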(event Custom|GlideTick
  (Utilities|FlowControl|Sequence
    (:then_0
      (bind _as角色 (Utilities|Casting|CastToCharacter (Ability|GetAvatarActorfromActorInfo))))
    (:then_1
      (if (< (.Z (Math|Vector|BreakVector (Variables|/Script/Engine.CharacterMovementComponent|GetVelocity (Actor|GetComponentbyClass _as角色 "/Script/Engine.CharacterMovementComponent")))) -1e+02)
        (Variables|/Script/Engine.CharacterMovementComponent|SetVelocity (Actor|GetComponentbyClass _as角色 "/Script/Engine.CharacterMovementComponent") (Math|Vector|MakeVector (.X (Math|Vector|BreakVector (Variables|/Script/Engine.CharacterMovementComponent|GetVelocity (Actor|GetComponentbyClass _as角色 "/Script/Engine.CharacterMovementComponent")))) (.Y (Math|Vector|BreakVector (Variables|/Script/Engine.CharacterMovementComponent|GetVelocity (Actor|GetComponentbyClass _as角色 "/Script/Engine.CharacterMovementComponent")))) -1e+02))
        (CallFunction|GlideTickApply)
        (else
          (CallFunction|GlideTickApply))))))

(event Custom|GlideTickApply
  (Ability|ApplyGameplayEffectToOwner "/Game/Tasks/gp-glide-stamina-bp/GE_GlideDrain.GE_GlideDrain_C")
  (if (<= (.ReturnValue (Ability|Attribute|GetFloatAttribute (Ability|GetAvatarActorfromActorInfo) "(AttributeName=\"Power\",Attribute=/Script/ThirdPerson.CraftBenchAttributeSet:Power,AttributeOwner=None)")) 0.0)
    (Ability|EndAbility)))

(event Ability|EventActivateAbility
  (bind _returnvalue (Ability|CommitAbility))
  (if _returnvalue
    (bind _returnvalue_2 (Utilities|Time|SetTimerbyEvent (EventDispatchers|CreateEvent :!event Custom|GlideTick) 0.1 true))
    (Variables|Default|SetGlideTimerHandle _returnvalue_2)
    (else
      (Ability|EndAbility))))

(event Ability|EventOnEndAbility
  (params (bWasCancelled :type Boolean))
  (Utilities|Time|ClearandInvalidateTimerbyHandle (Variables|Default|GetGlideTimerHandle)))