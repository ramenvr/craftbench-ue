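; BP_NearActiveSectorController switches which World Partition sector is active, using runtime Data Layer states.
; Its ApplySectorRequest event sets the request's first two candidate layers to Unloaded, then sets the selected layer to Activated, all non-recursively.
; It then teleports the request's streaming source actor to the selected destination without sweeping.
; The request supplies the layers, actor and destination, so the controller makes no selection itself.
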(event EventApplySectorRequest
  (params (Request :type Near%20Active%20Sector%20Request%20Object%20Reference))
  (bind _returnvalue (Class|NearActiveSectorControllerBase|GetSectorDataLayerManager))
  (bind _candidatelayers (Variables|/Script/ThirdPerson.NearActiveSectorRequest|GetCandidateLayers Request))
  (DataLayers|SetDataLayerRuntimeState _returnvalue (Utilities|Array|Get(acopy) _candidatelayers) "Unloaded" false :!class /Script/Engine.DataLayerManager)
  (DataLayers|SetDataLayerRuntimeState _returnvalue (Utilities|Array|Get(acopy) _candidatelayers 1) "Unloaded" false :!class /Script/Engine.DataLayerManager)
  (DataLayers|SetDataLayerRuntimeState _returnvalue (Variables|/Script/ThirdPerson.NearActiveSectorRequest|GetSelectedLayer Request) "Activated" false :!class /Script/Engine.DataLayerManager)
  (Transformation|SetActorLocation (Variables|/Script/ThirdPerson.NearActiveSectorRequest|GetStreamingSourceActor Request) (Variables|/Script/ThirdPerson.NearActiveSectorRequest|GetSelectedDestination Request) false true))

(fn ConstructionScript)